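; BP_WidgetEphemera is an actor that places a clickable widget button inside an animated book to control it.
; On BeginPlay it finds its parent BP_AnimatedBook and passes that reference, function, page settings and label to its W_WidgetButton, defaulting the label to the function name.
; It then flags its own entry in the book's Ephemera array as a non-flattening menu widget.
; The construction script sets widget facing and draw size.
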(event `self.ReceiveBeginPlay`
  (bind _my_widgetbutton (`self.My WidgetButton`))
  (bind _buttonlabeltext (`self.ButtonLabelText`))
  (bind _ephemera (`/Game/AnimatedBooks/Blueprints/BP_AnimatedBook.Ephemera` (`self.Book To Control`)))
  (`|ExecutionSequence`
    (:`then_0`
      ;[1 1 1] Find the AnimatedBook that owns me
      (bind _asbp_animated_book (cast `/Game/AnimatedBooks/Blueprints/BP_AnimatedBook` (`self.GetAttachParentActor`)) ; Get reference to the book I am in
        (:`then`
          (set `self.Book To Control` _asbp_animated_book))
        (:`CastFailed`
          (`KismetSystemLibrary.PrintString` "BP_MenuEphemera actor is not part of an AnimatedBook as expected" true true (struct :`G` 0.372801 :`B` 1.0 :`A` 1.0))))
      ;[1 1 1] Pass my Owner Book info to my Widget Component
      (bind _asw_widget_button (cast `/Game/AnimatedBooks/Blueprints/UMG/W_WidgetButton` (`WidgetComponent.GetUserWidgetObject` (`self.Widget`)))
        (:`then`
          (bind _output_get (set `self.My WidgetButton` _asw_widget_button))
          (set `/Game/AnimatedBooks/Blueprints/UMG/W_WidgetButton.BookToControl` (`self.Book To Control`) _output_get)
          ;[1 1 1] Set Widget Button's Function And Label
          (set `/Game/AnimatedBooks/Blueprints/UMG/W_WidgetButton.Button Function` (`self.Button Function`) _my_widgetbutton)
          (set `/Game/AnimatedBooks/Blueprints/UMG/W_WidgetButton.Page number` (`self.Page number`) _my_widgetbutton)
          (set `/Game/AnimatedBooks/Blueprints/UMG/W_WidgetButton.Open Book Amount` (`self.Open Book Amount`) _my_widgetbutton)
          (`TextBlock.SetText` (`/Game/AnimatedBooks/Blueprints/UMG/W_WidgetButton.ButtonLabelText` _my_widgetbutton) (select `bool` (`KismetTextLibrary.TextIsEmpty` _buttonlabeltext) :`false` _buttonlabeltext :`true` (`KismetTextLibrary.Conv_StringToText` (`|GetEnumeratorNameAsString` (`self.Button Function`))))))
        (:`CastFailed`
          (`KismetSystemLibrary.PrintString` "Cast Failed" true true (struct :`R` 1.0 :`B` 0.014997 :`A` 1.0) 10.0))))
    (:`then_1`
      (`/Engine/EditorBlueprintResources/StandardMacros.IsValid` (`self.Book To Control`)
        (:`Is Valid`
          ;[1 1 1] Ensure the Ephemera Settings in my parent book have me set to UI
          (for (_array_element _array_index) _ephemera
            (if (== (`.Actor_25_CB9E98F44229E223BCBAD7AEE2C3B438` (break `/Game/AnimatedBooks/Blueprints/Struct/S_Ephemera` _array_element)) self)
              (bind _structout (setmembers `/Game/AnimatedBooks/Blueprints/Struct/S_Ephemera` :`StructRef` _array_element :`Flatten between pages` false :`UseAsMenuWidget` true))
              (`KismetArrayLibrary.Array_Set` _ephemera _array_index _structout)
              (break))))))))

(fn `UserConstructionScript`
  (bind _widget (`self.Widget`))
  (`SceneComponent.K2_AddLocalRotation` _widget (select `bool` (`self.Face Reverse Direction`) :`true` (struct :`Yaw` 180.0) :!type "Rotator Structure") false false)
  (`WidgetComponent.SetDrawSize` _widget (`self.Widget Draw Size`)))