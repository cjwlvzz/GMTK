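; Demo controller actor that lets the player view and operate animated books, cycling through a library of them.
; A trigger volume or manual event either flies the book to the camera or blends to a close-up camera, optionally showing hints and a cursor.
; Keys turn pages, jump randomly and adjust openness.
; Timelines drive book moves and per-spread view offsets, while Tick handles scroll, zoom and slight close-up parallax from pawn movement.
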(event `Key|Q`
  (params (Key :type "Key Structure"))
  (bind _booktocontrol (`self.BookToControl`))
  ;[0 1 0.03201] BOOK CONTROLS
  ;
  ; You'll Probably Want To Edit These
  (:`Pressed`
    (if (< (`/Game/AnimatedBooks/Blueprints/BP_AnimatedBook.BookOpen_TargetAmount` (`self.BookToControl`)) 0.2)
      (if (< (`/Game/AnimatedBooks/Blueprints/BP_AnimatedBook.BookOpenCurrentAmount` _booktocontrol) 0.2) :!label _label
        (`/Game/AnimatedBooks/Blueprints/BP_AnimatedBook.Open To Page` _booktocontrol (`self.OpenBookHowWide`) 0.5 (- (`KismetArrayLibrary.Array_Length` (`/Game/AnimatedBooks/Blueprints/BP_AnimatedBook.Individual Pages` _booktocontrol)) 1)) ; open book to last page
        (else
          (`KismetSystemLibrary.Delay` 0.1) ; If necessary, wait until book is (mostly) closed
          (goto _label)))
      (else
        (`/Game/AnimatedBooks/Blueprints/BP_AnimatedBook.TurnThePage` (`self.BookToControl`) true (`self.PageTurnDuration`)) ; turn page to previous page
      ))
    (`self.CameraOffsetPerPage` false :!label _label_2) ; Check if any camera adjustments are requested
  ))

(event `Key|E`
  (params (Key :type "Key Structure"))
  (bind _booktocontrol (`self.BookToControl`))
  ;[0 1 0.03201] BOOK CONTROLS
  ;
  ; You'll Probably Want To Edit These
  (:`Pressed`
    (if (< (`/Game/AnimatedBooks/Blueprints/BP_AnimatedBook.BookOpen_TargetAmount` _booktocontrol) 0.2)
      (if (< (`/Game/AnimatedBooks/Blueprints/BP_AnimatedBook.BookOpenCurrentAmount` _booktocontrol) 0.2) :!label _label_3
        (`/Game/AnimatedBooks/Blueprints/BP_AnimatedBook.Open To Page` (`self.BookToControl`) (`self.OpenBookHowWide`) 1.0 1) ; open book to first page
        (goto _label_2)
        (else
          (`KismetSystemLibrary.Delay` 0.1) ; If necessary, wait until book is (mostly) closed
          (goto _label_3)))
      (else
        (`/Game/AnimatedBooks/Blueprints/BP_AnimatedBook.TurnThePage` (`self.BookToControl`) false (`self.PageTurnDuration`)) ; turn page to next page
        (goto _label_2)))))

(event `Key|R`
  (params (Key :type "Key Structure"))
  (bind _booktocontrol (`self.BookToControl`))
  ;[0 1 0.03201] BOOK CONTROLS
  ;
  ; You'll Probably Want To Edit These
  (:`Pressed`
    (`/Game/AnimatedBooks/Blueprints/BP_AnimatedBook.JumpToPage` _booktocontrol (`KismetMathLibrary.RandomIntegerInRange` 0 (- (`KismetArrayLibrary.Array_Length` (`/Game/AnimatedBooks/Blueprints/BP_AnimatedBook.Individual Pages` _booktocontrol)) 1)) 0.5) ; jump to whatever page number is given
    (goto _label_2)))

(event `Key|F`
  (params (Key :type "Key Structure"))
  (bind _booktocontrol (`self.BookToControl`))
  (bind _returnvalue (+ (`/Game/AnimatedBooks/Blueprints/BP_AnimatedBook.BookOpen_TargetAmount` _booktocontrol) 0.34))
  ;[0 1 0.03201] BOOK CONTROLS
  ;
  ; You'll Probably Want To Edit These
  (:`Pressed`
    (`/Game/AnimatedBooks/Blueprints/BP_AnimatedBook.Open To Page` _booktocontrol (`KismetMathLibrary.SelectFloat` 1.0 _returnvalue (>= _returnvalue 1.0)) 0.5 -1) ; Opening to the already-open page (page number -1) but changing the\n"Open how wide" value allows you to adjust how open the book is.
    (goto _label_2)))

(event `Key|G`
  (params (Key :type "Key Structure"))
  (bind _booktocontrol (`self.BookToControl`))
  (bind _returnvalue (- (`/Game/AnimatedBooks/Blueprints/BP_AnimatedBook.BookOpen_TargetAmount` _booktocontrol) 0.34))
  ;[0 1 0.03201] BOOK CONTROLS
  ;
  ; You'll Probably Want To Edit These
  (:`Pressed`
    (`/Game/AnimatedBooks/Blueprints/BP_AnimatedBook.Open To Page` _booktocontrol (`KismetMathLibrary.SelectFloat` 0.0 _returnvalue (<= _returnvalue 0.0)) 0.5 -1) ; Opening to the already-open page (page number -1) but changing the\n"Open how wide" value allows you to adjust how open the book is.
    (goto _label_2)))

(event `Key|Equals`
  (params (Key :type "Key Structure"))
  (bind _returnvalue (+ (`self.CurrentBook`) 1))
  ;[0 1 0.03201] BOOK CONTROLS
  ;
  ; You'll Probably Want To Edit These
  (:`Pressed`
    (if (> (`KismetArrayLibrary.Array_Length` (`self.BooksToControl`)) 1)
      (if (`self.BringBookToPlayer`)
        (`self.MoveBookToPlayer` true)
        (else
          (`/Engine/EditorBlueprintResources/StandardMacros.IsValid` (`self.CloseUpCamera`)
            (:`Is Valid`
              (`self.MoveViewToTarget` true))
            (:`Is Not Valid`
              _))))
      (`KismetSystemLibrary.Delay` (`self.TransitionTime`))
      (set `self.CurrentBook` (select `bool` (> (`KismetArrayLibrary.Array_Length` (`self.BooksToControl`)) _returnvalue) :`true` _returnvalue))
      (set `self.BookToControl` (`|GetArrayItem` (`self.BooksToControl`) (`self.CurrentBook`)) :!label _label_4)
      (`SceneComponent.K2_SetWorldTransform` (`self.OriginLocation`) (`self.GetTransform` (`self.BookToControl`)) false true)
      (`SceneComponent.K2_SetWorldTransform` (`self.CloseUpCamMount`) (`self.GetTransform` (`self.BookToControl`)) false true)
      (if (`self.BringBookToPlayer`)
        (`self.MoveBookToPlayer` false)
        (else
          (`/Engine/EditorBlueprintResources/StandardMacros.IsValid` (`self.CloseUpCamera`)
            (:`Is Valid`
              (`self.MoveViewToTarget` false))))))))

(event `Key|Hyphen`
  (params (Key :type "Key Structure"))
  (bind _returnvalue (- (`self.CurrentBook`) 1))
  ;[0 1 0.03201] BOOK CONTROLS
  ;
  ; You'll Probably Want To Edit These
  (:`Pressed`
    (if (> (`KismetArrayLibrary.Array_Length` (`self.BooksToControl`)) 1)
      (if (`self.BringBookToPlayer`)
        (`self.MoveBookToPlayer` true)
        (else
          (`/Engine/EditorBlueprintResources/StandardMacros.IsValid` (`self.CloseUpCamera`)
            (:`Is Valid`
              (`self.MoveViewToTarget` true))
            (:`Is Not Valid`
              _))))
      (`KismetSystemLibrary.Delay` (`self.TransitionTime`))
      (set `self.CurrentBook` (select `bool` (<= 0 _returnvalue) :`false` (- (`KismetArrayLibrary.Array_Length` (`self.BooksToControl`)) 1) :`true` _returnvalue))
      (goto _label_4))))

(event `Key|MouseScrollUp` :consume false
  (params (Key :type "Key Structure"))
  ;[0 1 0.03201] BOOK CONTROLS
  ;
  ; You'll Probably Want To Edit These
  (:`Pressed`
    (set `self.ZoomAmount` (`KismetMathLibrary.FClamp` (+ (`self.ZoomAmount`) 0.08)))
    (set `self.ZoomCurrent` (* (`self.ZoomAmount`) (`self.ZoomMax`)) :!label _label_5)))

(event `Key|MouseScrollDown` :consume false
  (params (Key :type "Key Structure"))
  ;[0 1 0.03201] BOOK CONTROLS
  ;
  ; You'll Probably Want To Edit These
  (:`Pressed`
    (set `self.ZoomAmount` (`KismetMathLibrary.FClamp` (- (`self.ZoomAmount`) 0.08)))
    (goto _label_5)))

(event `Key|F10`
  (params (Key :type "Key Structure"))
  ;[0 1 0.03201] BOOK CONTROLS
  ;
  ; You'll Probably Want To Edit These
  (:`Pressed`
    (`KismetSystemLibrary.ExecuteConsoleCommand` "Shot" null)))

(event `Key|LeftMouseButton`
  (params (Key :type "Key Structure"))
  (bind _widgetinteraction (`self.WidgetInteraction`))
  ;[0 1 0.03201] BOOK CONTROLS
  ;
  ; You'll Probably Want To Edit These
  (:`Pressed`
    (`WidgetInteractionComponent.PressPointerKey` _widgetinteraction "LeftMouseButton") ; Send mouse clicks to any widget buttons via Widget Interaction component
  )
  (:`Released`
    (`WidgetInteractionComponent.ReleasePointerKey` _widgetinteraction "LeftMouseButton")))

(event `self.ReceiveBeginPlay`
  (bind _destinationlocation (`self.DestinationLocation`))
  (set `self.BookToControl` (`|GetArrayItem` (`self.BooksToControl`) (`self.CurrentBook`)))
  (if (not (`self.RequirePlayerInsideTriggerVolume`))
    (`self.EnableInput` (`GameplayStatics.GetPlayerController` 0)) ; Listen for player input to control book
  )
  (if (`self.BringBookToPlayer`)
    (`SceneComponent.K2_AttachToComponent` (`self.DestinationLocation`) (`Actor.RootComponent` (`GameplayStatics.GetPlayerCameraManager` 0)) "None" "SnapToTarget" "SnapToTarget" "KeepRelative" false)
    (`SceneComponent.K2_AddLocalOffset` _destinationlocation (`KismetMathLibrary.MakeVector` (.z (select `bool` (`HeadMountedDisplayFunctionLibrary.IsHeadMountedDisplayEnabled`) :`false` (`self.DistanceFromCamera`) :`true` (`self.DistanceFromCameraVR`))) (.x (select `bool` (`HeadMountedDisplayFunctionLibrary.IsHeadMountedDisplayEnabled`) :`false` (`self.DistanceFromCamera`) :`true` (`self.DistanceFromCameraVR`))) (.y (select `bool` (`HeadMountedDisplayFunctionLibrary.IsHeadMountedDisplayEnabled`) :`false` (`self.DistanceFromCamera`) :`true` (`self.DistanceFromCameraVR`)))) false true)
    (`SceneComponent.K2_AddLocalRotation` _destinationlocation (`self.Book Viewing Angle`) false false)
    (`SceneComponent.K2_SetWorldTransform` (`self.OriginLocation`) (`self.GetTransform` (`self.BookToControl`)) false true)
    (`SceneComponent.K2_SetWorldTransform` (`self.CloseUpCamMount`) (`self.GetTransform` (`self.BookToControl`)) false true)
    (else
      (`/Engine/EditorBlueprintResources/StandardMacros.IsValid` (`self.CloseUpCamera`)
        (:`Is Valid`
          (`SceneComponent.K2_SetWorldTransform` (`self.OriginLocation`) (`SceneComponent.K2_GetComponentToWorld` (`Actor.RootComponent` (`self.CloseUpCamera`))) false true)
          (`SceneComponent.K2_SetWorldTransform` (`self.CloseUpCamMount`) (`SceneComponent.K2_GetComponentToWorld` (`Actor.RootComponent` (`self.CloseUpCamera`))) false true)
          (`self.K2_AttachToComponent` (`self.CloseUpCamera`) (`self.CloseUpCamMount`) "None" "SnapToTarget" "SnapToTarget" "SnapToTarget" true))
        (:`Is Not Valid`
          (set `self.DoNothing` true)))))
  (set `self.BookOriginalOpenAmount` (`/Game/AnimatedBooks/Blueprints/BP_AnimatedBook.BookOpen_TargetAmount` (`self.BookToControl`)))
  (`TimelineComponent.SetPlayRate` (`self.MoveToCamera`) 1.5)
  (bind _returnvalue (`|CreateWidget` "/Game/AnimatedBooks/Blueprints/UMG/W_TutorialHints.W_TutorialHints_C"))
  (set `self.TutorialWidget` _returnvalue)
  (`TimelineComponent.SetPlayRate` (`self.OffsetPerPage`) (/ 1.0 (`self.TransitionTimeForOffsets`)))
  (`TimelineComponent.SetPlayRate` (`self.MoveToCamera`) (/ 1.0 (`self.TransitionTime`))))

(event `ManuallyTriggerController`
  (bind _returnvalue (`GameplayStatics.GetPlayerController` 0))
  (bind _returnvalue_2 (`GameplayStatics.GetPlayerController` 0))
  (bind _tutorialwidget (`self.TutorialWidget`))
  (bind _widgetinteraction (`self.WidgetInteraction`))
  (bind _bookopeninginprogress (`/Game/AnimatedBooks/Blueprints/BP_AnimatedBook.BookOpeningInProgress` (`self.BookToControl`)))
  (bind _returnvalue_3 (and (`self.Show Controls UI`) (not (`HeadMountedDisplayFunctionLibrary.IsHeadMountedDisplayEnabled`))))
  ;[0 1 0.03201] Manual Override
  (`/Engine/EditorBlueprintResources/StandardMacros.FlipFlop`
    (:`A`
      (if (not (`self.TriggerActivated`)) :!label _label_6
        (set `self.TriggerActivated` true)
        (if (`self.RequirePlayerInsideTriggerVolume`)
          (`self.EnableInput` _returnvalue) ; Listen for player input to control book
        )
        (if (`self.BringBookToPlayer`)
          (set `self.waiting` false)
          (if _bookopeninginprogress :!label _label_7
            (set `self.waiting` true)
            (`KismetSystemLibrary.Delay` 0.2)
            (if (`self.waiting`)
              (goto _label_7))
            (else
              (`self.MoveBookToPlayer` false)
              ;[0.125 0.125 0.125] Show Hint Text?
              (if _returnvalue_3 :!label _label_8
                (if (not (`Widget.IsInViewport` _tutorialwidget))
                  (`UserWidget.AddToViewport` _tutorialwidget 0) ; Add Hint Text to screen
                ))
              ;[0.125 0.125 0.125] Switch to (Widget Buttons) UI input mode?
              (if (`self.EnableMouseCursor`)
                (`WidgetBlueprintLibrary.SetInputMode_GameAndUIEx` _returnvalue_2 null "LockAlways" false)
                (set `PlayerController.bShowMouseCursor` true _returnvalue_2)
                (`ActorComponent.Activate` _widgetinteraction false))))
          (elif (`self.DoNothing`)
            (goto _label_8)
            (else
              (`self.MoveViewToTarget` false)
              (goto _label_8))))))
    (:`B`
      (if (`self.TriggerActivated`) :!label _label_9
        (set `self.TriggerActivated` false)
        (if (`self.RequirePlayerInsideTriggerVolume`)
          (`self.DisableInput` _returnvalue) ; Stop listening to player input to control book
        )
        (if (`self.BringBookToPlayer`)
          (set `self.waiting` false)
          (if _bookopeninginprogress :!label _label_10
            (set `self.waiting` true)
            (`KismetSystemLibrary.Delay` 0.2)
            (if (`self.waiting`)
              (goto _label_10))
            (else
              (`self.MoveBookToPlayer` true)
              (if _returnvalue_3 :!label _label_11
                (`Widget.RemoveFromParent` _tutorialwidget))
              ;[0.125 0.125 0.125] Reset Page Animations?
              (if (`self.ResetAnimsOnBookReturn`)
                (`/Game/AnimatedBooks/Blueprints/BP_AnimatedBook.Reset Text Animation` (`self.BookToControl`) 0 true))
              (if (`self.EnableMouseCursor`)
                (`WidgetBlueprintLibrary.SetInputMode_GameOnly` _returnvalue_2)
                (set `PlayerController.bShowMouseCursor` false _returnvalue_2)
                (`ActorComponent.Deactivate` _widgetinteraction))
              ;[0.125 0.125 0.125] Reset Zoom
              (`KismetSystemLibrary.Delay` (`self.TransitionTime`))
              (if (`self.MoveEnded`)
                (set `self.ZoomAmount` 0.0) ; Reset zoom amount if transition has ended and player has left area
                (set `self.ZoomCurrent` 0.0))))
          (elif (`self.DoNothing`)
            (goto _label_11)
            (else
              (`self.MoveViewToTarget` true)
              (goto _label_11))))))))

(event `self.TriggerVolume.OnComponentBeginOverlap`
  (params (OverlappedComponent :type "PrimitiveComponent Object Reference") (OtherActor :type "Actor Object Reference") (OtherComp :type "PrimitiveComponent Object Reference") (OtherBodyIndex :type Integer) (bFromSweep :type Boolean) (SweepResult :type "HitResult Structure (by ref)"))
  (if (== OtherComp (`Actor.RootComponent` (`GameplayStatics.GetPlayerPawn` 0)))
    (goto _label_6)))

(event `self.TriggerVolume.OnComponentEndOverlap`
  (params (OverlappedComponent :type "PrimitiveComponent Object Reference") (OtherActor :type "Actor Object Reference") (OtherComp :type "PrimitiveComponent Object Reference") (OtherBodyIndex :type Integer))
  (if (== (`Actor.RootComponent` (`GameplayStatics.GetPlayerPawn` 0)) OtherComp)
    (goto _label_9)))

(event `MoveBookToPlayer`
  (params (ReturnBook :type Boolean))
  (bind _booktocontrol (`self.BookToControl`))
  (if (`self.EnableZoomAndScroll`)
    (`self.SetActorTickEnabled` (not ReturnBook)) ; Only enable tick when mouse input is needed
  )
  (bind _output_get (set `self.MoveEnded` ReturnBook))
  (`/Game/AnimatedBooks/Blueprints/BP_AnimatedBook.Open To Page` (`self.BookToControl`) (`KismetMathLibrary.SelectFloat` (`self.BookOriginalOpenAmount`) (`self.OpenBookHowWide`) (or ReturnBook (not (`self.Auto-open book upon viewing`)))) 0.7 (select `bool` ReturnBook :`false` (`self.PageToOpenTo`) :`true` -1))
  (set `self.MoveBookActive` true)
  (if _output_get
    (bind (_direction _sine0_1) (`Timeline|MoveToCamera` :!via `Reverse` :!label _label_12)
      (:`Update`
        (`self.K2_SetActorTransform` (`self.BookToControl`) (`KismetMathLibrary.MakeTransform` (.location (`KismetMathLibrary.TLerp` (`SceneComponent.K2_GetComponentToWorld` (`self.OriginLocation`)) (`SceneComponent.K2_GetComponentToWorld` (`self.OffsetLocation`)) _sine0_1)) (.rotation (`KismetMathLibrary.TLerp` (`SceneComponent.K2_GetComponentToWorld` (`self.OriginLocation`)) (`SceneComponent.K2_GetComponentToWorld` (`self.OffsetLocation`)) _sine0_1)) (`self.GetActorScale3D` (`self.BookToControl`))) false true))
      (:`Finished`
        (set `self.MoveBookActive` false)
        (if _output_get
          (`self.K2_DetachFromActor` _booktocontrol "KeepWorld" "KeepWorld" "KeepWorld")
          (`self.CameraOffsetPerPage` true)
          (else
            (`self.K2_AttachToComponent` _booktocontrol (`self.DestinationLocation`) "None" "KeepWorld" "KeepWorld" "KeepWorld" false)
            (`self.CameraOffsetPerPage` false)))))
    (else
      (goto _label_12))))

(event `MoveViewToTarget`
  (params (Return :type Boolean))
  (bind _returnvalue (`GameplayStatics.GetPlayerController` 0))
  (bind _transitiontime (`self.TransitionTime`))
  (set `self.MoveEnded` Return)
  (`self.SetActorTickEnabled` (not Return)) ; only enable tick when mouse input is needed
  (if Return
    (`PlayerController.SetViewTargetWithBlend` _returnvalue (`Controller.K2_GetPawn` _returnvalue) _transitiontime "VTBlend_Cubic" 1.0 false)
    (`self.CameraOffsetPerPage` true)
    (else
      (`PlayerController.SetViewTargetWithBlend` _returnvalue (`self.CloseUpCamera`) _transitiontime "VTBlend_Cubic" 1.0 false)
      (`self.CameraOffsetPerPage` false))))

(event `CameraOffsetPerPage`
  (params (halt :type Boolean))
  (bind _cameraoffsetsbypagespread (`self.CameraOffsetsByPageSpread`))
  (bind _offsetlocation (`self.OffsetLocation`))
  (bind _returnvalue (select `bool` (< (`/Game/AnimatedBooks/Blueprints/BP_AnimatedBook.BookOpen_TargetAmount` (`self.BookToControl`)) 0.2) :`false` (`/Game/AnimatedBooks/Blueprints/BP_AnimatedBook.CurrentPage` (`self.BookToControl`))))
  (bind (_value _returnvalue_2) (`BlueprintMapLibrary.Map_Find` _cameraoffsetsbypagespread _returnvalue))
  (bind (_value_2 _returnvalue_3) (`BlueprintMapLibrary.Map_Find` _cameraoffsetsbypagespread (- _returnvalue 1)))
  (if halt
    (bind (_direction _0_1) (`Timeline|OffsetPerPage` :!via `Stop` :!label _label_13)
      (:`Update`
        (if (`self.BringBookToPlayer`)
          (bind _returnvalue_4 (`KismetMathLibrary.TLerp` (`SceneComponent.K2_GetComponentToWorld` (`self.OffsetStartLocation`)) (`SceneComponent.K2_GetComponentToWorld` (`self.OffsetLocation`)) _0_1))
          (`self.K2_SetActorTransform` (`self.BookToControl`) (`KismetMathLibrary.MakeTransform` (.location _returnvalue_4) (.rotation _returnvalue_4) (`self.GetActorScale3D` (`self.BookToControl`))) false true)
          (else
            (`SceneComponent.K2_SetWorldTransform` (`self.CloseUpCamMount`) _returnvalue_4 false false))))
      (:`Finished`
        (set `self.MoveViewActive` false)))
    (else
      (`TimelineComponent.SetPlayRate` (`self.OffsetPerPage`) (/ 1.0 (`self.TransitionTimeForOffsets`)))
      (`KismetSystemLibrary.Delay` (* (`self.PageTurnDuration`) 0.5))
      (if (`self.MoveEnded`) :!label _label_14
        (goto _label_13 :!via `Stop`)
        (elif (`/Game/AnimatedBooks/Blueprints/BP_AnimatedBook.PageTurnQueued` (`self.BookToControl`))
          (`KismetSystemLibrary.Delay` 0.2)
          (goto _label_14)
          (else
            (bind _output_get (set `self.LocationStart` (select `bool` (`self.BringBookToPlayer`) :`false` (`SceneComponent.K2_GetComponentToWorld` (`self.CloseUpCamMount`)) :`true` (`self.GetTransform` (`self.BookToControl`)))))
            (`SceneComponent.K2_SetWorldTransform` (`self.OffsetStartLocation`) _output_get false true)
            (`SceneComponent.K2_SetWorldTransform` _offsetlocation (select `bool` (`self.BringBookToPlayer`) :`false` (`SceneComponent.K2_GetComponentToWorld` (`self.OriginLocation`)) :`true` (`SceneComponent.K2_GetComponentToWorld` (`self.ScrollAndZoomOffset`))) false true)
            (`SceneComponent.K2_AddLocalTransform` _offsetlocation (`KismetMathLibrary.SelectTransform` _value (`KismetMathLibrary.SelectTransform` _value_2 (`KismetMathLibrary.MakeTransform` (0.0 0.0 0.0)) _returnvalue_3) _returnvalue_2) false true)
            (set `self.MoveViewActive` true)
            (goto _label_13 :!via `PlayFromStart`)))))))

(event `self.ReceiveTick`
  (params (DeltaSeconds :type "Float (single-precision)"))
  (bind _offsetzoompos (`self.OffsetZoomPos`))
  (bind _zoomamount (`self.ZoomAmount`))
  (bind _zoomamount_2 (`self.ZoomAmount`))
  (bind _offsetzoompos_2 (`self.OffsetZoomPos`))
  (bind (_left _top _right _bottom) (break `Margin` (`self.ScrollMax`)))
  (bind (_left_2 _top_2 _right_2 _bottom_2) (break `Margin` (`self.ScrollMax`)))
  (bind (_left_3 _top_3 _right_3 _bottom_3) (break `Margin` (`self.ScrollMax`)))
  (bind (_left_4 _top_4 _right_4 _bottom_4) (break `Margin` (`self.ScrollMax`)))
  (bind _returnvalue (`KismetMathLibrary.MakeVector` (`self.GetInputAxisKeyValue`) (`self.GetInputAxisKeyValue`)))
  (bind _returnvalue_2 (`KismetMathLibrary.MakeVector` 0.0 (`self.GetInputAxisKeyValue`) (`self.GetInputAxisKeyValue`)))
  (bind _x (.x (select `bool` (`self.InvertScrolling`) :`false` (- _offsetzoompos _returnvalue) :`true` (+ _offsetzoompos _returnvalue))))
  (bind _y (.y (select `bool` (`self.InvertScrolling`) :`false` (- _offsetzoompos _returnvalue) :`true` (+ _offsetzoompos _returnvalue))))
  (bind _y_2 (.y (select `bool` (`self.InvertScrolling`) :`false` (+ _offsetzoompos_2 _returnvalue_2) :`true` (- _offsetzoompos_2 _returnvalue_2))))
  (bind _z (.z (select `bool` (`self.InvertScrolling`) :`false` (+ _offsetzoompos_2 _returnvalue_2) :`true` (- _offsetzoompos_2 _returnvalue_2))))
  (bind _returnvalue_3 (`KismetMathLibrary.MakeVector` (.x (* (- (`self.K2_GetActorLocation` (`GameplayStatics.GetPlayerPawn` 0)) (`self.K2_GetActorLocation` self)) (`self.CloseUpCamMovementMultiplier`))) (.y (* (- (`self.K2_GetActorLocation` (`GameplayStatics.GetPlayerPawn` 0)) (`self.K2_GetActorLocation` self)) (`self.CloseUpCamMovementMultiplier`)))))
  (if (`self.BringBookToPlayer`)
    (bind _output_get (set `self.OffsetZoomPos` (`KismetMathLibrary.SelectVector` (`KismetMathLibrary.MakeVector` (`KismetMathLibrary.FClamp` _x (* _bottom_3 -1.0 _zoomamount) (* _top_3 _zoomamount)) (`KismetMathLibrary.FClamp` _y (* _left_3 -1.0 _zoomamount) (* _right_3 _zoomamount))) (`KismetMathLibrary.MakeVector` (`KismetMathLibrary.FClamp` _x (* _bottom -1.0) _top) (`KismetMathLibrary.FClamp` _y (* _left -1.0) _right)) (`self.LimitScrollToZoom`)))) ; offset created by view-scrolling
    (bind _output_get_2 (set `self.OffsetTotalPos` (+ _output_get (`KismetMathLibrary.MakeVector` 0.0 0.0 (`self.ZoomCurrent`))))) ; total offset
    (`SceneComponent.K2_SetRelativeLocation` (`self.ScrollAndZoomOffset`) _output_get_2 false false)
    (if (`KismetMathLibrary.BooleanNOR` (`self.MoveBookActive`) (`self.MoveViewActive`))
      (`self.K2_SetActorTransform` (`self.BookToControl`) (`KismetMathLibrary.MakeTransform` (.location (`SceneComponent.K2_GetComponentToWorld` (`self.OffsetLocation`))) (.rotation (`SceneComponent.K2_GetComponentToWorld` (`self.OffsetLocation`))) (`self.GetActorScale3D` (`self.BookToControl`))) false true))
    (else
      (bind _output_get_3 (set `self.OffsetZoomPos` (`KismetMathLibrary.SelectVector` (`KismetMathLibrary.MakeVector` 0.0 (`KismetMathLibrary.FClamp` _y_2 (* _left_4 -1.0 _zoomamount_2) (* _right_4 _zoomamount_2)) (`KismetMathLibrary.FClamp` _z (* _bottom_4 -1.0 _zoomamount_2) (* _top_4 _zoomamount_2))) (`KismetMathLibrary.MakeVector` 0.0 (`KismetMathLibrary.FClamp` _y_2 (* _left_2 -1.0) _right_2) (`KismetMathLibrary.FClamp` _z (* _bottom_2 -1.0) _top_2)) (`self.LimitScrollToZoom`)))) ; offset created by view-scrolling
      (bind _output_get_4 (set `self.OffsetTotalPos` (select `bool` (`self.EnableZoomAndScroll`) :`false` _returnvalue_3 :`true` (+ (`KismetMathLibrary.GreaterGreater_VectorRotator` (+ _output_get_3 (`KismetMathLibrary.MakeVector` (`self.ZoomCurrent`))) (`self.K2_GetActorRotation` (`self.CloseUpCamera`))) _returnvalue_3)))) ; total offset
      (`self.K2_SetActorLocation` (`self.CloseUpCamera`) (+ _output_get_4 (`SceneComponent.K2_GetComponentLocation` (`self.CloseUpCamMount`))) false true) ; Make ZoomCam respond SLIGHTLY to changes in player position\nPlus respond to scroll/zoom input
    )))

(fn `UserConstructionScript`
  (`SceneComponent.SetWorldScale3D` (`self.TriggerVolume`) (`self.Trigger Volume Dimensions`))
  (if (<= (`self.TransitionTimeForOffsets`) 0.0)
    (set `self.TransitionTimeForOffsets` 0.001))
  (if (<= (`self.TransitionTime`) 0.0)
    (set `self.TransitionTime` 0.001)))