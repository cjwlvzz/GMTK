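; BP_BlockType1 is a block actor that the player drags over a grid with the cursor.
; Pressing the block starts following and releasing stops it; while following, Tick moves it to the cursor's hit location.
; A short line trace along the block's up vector finds the grid mesh, tints it through a dynamic material instance, and records it as GridGenerator's current selection before calling UpdateMat.
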(event `self.ReceiveBeginPlay`
  (`parent.ReceiveBeginPlay`))

(event `self.Block.OnReleased`
  (params (TouchedComponent :type "PrimitiveComponent Object Reference") (ButtonReleased :type "Key Structure"))
  (set `self.ShouldFollow` false))

(event `self.Block.OnClicked`
  (params (TouchedComponent :type "PrimitiveComponent Object Reference") (ButtonPressed :type "Key Structure"))
  (set `self.ShouldFollow` true))

(event `self.ReceiveTick`
  (params (DeltaSeconds :type "Float (single-precision)"))
  (bind _gridgenerator (`self.GridGenerator`))
  (bind _returnvalue (`SceneComponent.K2_GetComponentLocation` (`self.Block`)))
  (if (`self.ShouldFollow`)
    (`KismetArrayLibrary.Array_Clear` (`/Game/Core/BP_GridGenerating.CurrentSelectedMesh` (`self.GridGenerator`)))
    (`SceneComponent.K2_SetWorldLocation` (`self.Block`) (`.Location` (`GameplayStatics.BreakHitResult` (`PlayerController.GetHitResultUnderCursorByChannel` (`GameplayStatics.GetPlayerController` 0) "TraceTypeQuery3" true))) false false)
    (bind _outhit (`KismetSystemLibrary.LineTraceSingle` _returnvalue (+ _returnvalue (* (`SceneComponent.GetUpVector` (`self.Block`)) (50.0 50.0 50.0))) "TraceTypeQuery5"))
    (bind _asstatic_mesh_component (cast `StaticMeshComponent` (`.HitComponent` (`GameplayStatics.BreakHitResult` _outhit))))
    (`KismetArrayLibrary.Array_Add` (`/Game/Core/BP_GridGenerating.CurrentSelectedMesh` _gridgenerator) _asstatic_mesh_component)
    (bind _returnvalue_2 (`PrimitiveComponent.CreateDynamicMaterialInstance` _asstatic_mesh_component 0 "/Game/Source/Materials/GridShapes/MI_Grid_Flat_Border_Square.MI_Grid_Flat_Border_Square" "None"))
    (`MaterialInstanceDynamic.SetVectorParameterValue` _returnvalue_2 "Color" (struct :`R` 1.0 :`G` 0.69197 :`B` 0.335289 :`A` 1.0))
    (`/Game/Core/BP_GridGenerating.UpdateMat` _gridgenerator)))

(fn `UserConstructionScript`
  (`parent.UserConstructionScript`))