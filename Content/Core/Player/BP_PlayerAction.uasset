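; BP_PlayerAction routes the player's left and right mouse clicks to swappable tile actions.
; SetSelectedActions destroys the current action actor for each button and spawns one from the given class, passing itself as PlayerActions.
; BeginPlay enables input and assigns BP_ActionSelecTile to both buttons.
; Each click refreshes the tile under the cursor, then executes that button's action on HoveredTile.
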(event `self.ReceiveBeginPlay`
  (`self.EnableInput` (`GameplayStatics.GetPlayerController` 0))
  (`self.SetSelectedActions` "/Game/Core/Player/Actions/Grid/BP_ActionSelecTile.BP_ActionSelecTile_C" "/Game/Core/Player/Actions/Grid/BP_ActionSelecTile.BP_ActionSelecTile_C"))

(event `Key|LeftMouseButton`
  (params (Key :type "Key Structure"))
  (:`Pressed`
    (`self.UpdateTileUnderCursor`)
    (`/Engine/EditorBlueprintResources/StandardMacros.IsValid` (`self.SelectedAction_LeftClick`)
      (:`Is Valid`
        (`/Game/Core/Player/Actions/BP_Action.ExecuteAction` (`self.SelectedAction_LeftClick`) (`self.HoveredTile`))))))

(event `Key|RightMouseButton`
  (params (Key :type "Key Structure"))
  (:`Pressed`
    (`self.UpdateTileUnderCursor`)
    (`/Engine/EditorBlueprintResources/StandardMacros.IsValid` (`self.SelectedAction_RightClick`)
      (:`Is Valid`
        (`/Game/Core/Player/Actions/BP_Action.ExecuteAction` (`self.SelectedAction_RightClick`) (`self.HoveredTile`))))))

(fn `SetSelectedActions`
  (params (LeftActon :type "/Game/Core/Player/Actions/BP_Action Class Reference") (RightAction :type "/Game/Core/Player/Actions/BP_Action Class Reference"))
  (bind _selectedaction_leftclick (`self.SelectedAction_LeftClick`))
  (bind _selectedaction_rightclick (`self.SelectedAction_RightClick`))
  (`|ExecutionSequence`
    (:`then_0`
      (`/Engine/EditorBlueprintResources/StandardMacros.IsValid` _selectedaction_leftclick
        (:`Is Valid`
          (`self.K2_DestroyActor` _selectedaction_leftclick)
          (set `self.SelectedAction_LeftClick` null))
        (:`Is Not Valid`
          _))
      (if (`KismetSystemLibrary.IsValidClass` (`local.LeftActon`))
        (bind _returnvalue (`|SpawnActorFromClass` (`local.LeftActon`) (`KismetMathLibrary.MakeTransform` (0.0 0.0 0.0)) "AlwaysSpawn" "MultiplyWithRoot" null self null))
        (set `self.SelectedAction_LeftClick` _returnvalue)))
    (:`then_1`
      (`/Engine/EditorBlueprintResources/StandardMacros.IsValid` _selectedaction_rightclick
        (:`Is Valid`
          (`self.K2_DestroyActor` _selectedaction_rightclick)
          (set `self.SelectedAction_RightClick` null))
        (:`Is Not Valid`
          _))
      (if (`KismetSystemLibrary.IsValidClass` (`local.RightAction`))
        (bind _returnvalue_2 (`|SpawnActorFromClass` (`local.RightAction`) (`KismetMathLibrary.MakeTransform` (0.0 0.0 0.0)) "AlwaysSpawn" "MultiplyWithRoot" null self null))
        (set `self.SelectedAction_RightClick` _returnvalue_2)))))

(fn `UserConstructionScript`)