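; Player grid action that selects or deselects a tile.
; ExecuteAction moves the Selected state on the PlayerActions' Grid from the previous tile to the given index and stores it as SelectedTile.
; Executing on the already selected tile removes the state and resets SelectedTile to an out-of-range sentinel index.
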(event `self.ReceiveBeginPlay`
  (`parent.ReceiveBeginPlay`))

(fn `ExecuteAction`
  (params (Index :type "IntPoint Structure"))
  (bind _playeractions (`self.PlayerActions`))
  (bind _playeractions_2 (`self.PlayerActions`))
  (bind _playeractions_3 (`self.PlayerActions`))
  (if (!= (`PlayerAction.SelectedTile` (`self.PlayerActions`)) (`local.Index`))
    (`Grid.RemoveStateFromTile` (`PlayerAction.Grid` _playeractions_3) (`PlayerAction.SelectedTile` _playeractions_3) "Selected")
    (set `PlayerAction.SelectedTile` (`local.Index`) (`self.PlayerActions`))
    (`Grid.AddStateToTile` (`PlayerAction.Grid` _playeractions) (`PlayerAction.SelectedTile` _playeractions) "Selected")
    (else
      (`Grid.RemoveStateFromTile` (`PlayerAction.Grid` _playeractions_2) (`PlayerAction.SelectedTile` _playeractions_2) "Selected")
      (set `PlayerAction.SelectedTile` (make `IntPoint` -999 -999) (`self.PlayerActions`)))))

(fn `UserConstructionScript`
  (`parent.UserConstructionScript`))