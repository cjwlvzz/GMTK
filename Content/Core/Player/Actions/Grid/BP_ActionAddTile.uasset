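; Player grid action that adds a tile to the grid at a given index.
; ExecuteAction acts only when the grid reports that index as not valid.
; It then calls AddGridTile on the PlayerActions grid, building the tile's transform from the grid's own location, rotation and scale getters.
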(event `self.ReceiveBeginPlay`
  (`parent.ReceiveBeginPlay`))

(fn `ExecuteAction`
  (params (Index :type "IntPoint Structure"))
  (bind _index (`local.Index`))
  (bind _grid (`PlayerAction.Grid` (`self.PlayerActions`)))
  (if (not (`Grid.IsIndexValid` (`PlayerAction.Grid` (`self.PlayerActions`)) (`local.Index`)))
    (`Grid.AddGridTile` (`PlayerAction.Grid` (`self.PlayerActions`)) (make `TileData` (`local.Index`) "Normal" (`KismetMathLibrary.MakeTransform` (`Grid.GetTileLocationFromGridIndex` _grid _index) (`Grid.GetTileRotationFromGridIndex` _grid _index) (`Grid.GetTileScale` _grid))))))

(fn `UserConstructionScript`
  (`parent.UserConstructionScript`))