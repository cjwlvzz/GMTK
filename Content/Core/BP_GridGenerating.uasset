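; BP_GridGenerating is a grid actor made of pre-placed static mesh components, gathered into AllMeshes on BeginPlay.
; UpdateMat gives each mesh outside CurrentSelectedMesh a new dynamic instance of the flat border-square grid material, with Color set to black.
; Unconnected graph logic sketches a ShouldFollow toggle that moves to the cursor hit and debug-traces along the Grid mesh's up vector.
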(event `self.ReceiveTick`
  (params (DeltaSeconds :type "Float (single-precision)")))

(event `self.ReceiveBeginPlay`
  (set `self.AllMeshes` (`|MakeArray` (`self.StaticMesh4`) (`self.StaticMesh6`) (`self.StaticMesh7`) (`self.StaticMesh8`) (`self.StaticMesh9`) (`self.StaticMesh10`) (`self.StaticMesh5`) (`self.Grid`) (`self.StaticMesh`) (`self.StaticMesh1`) (`self.StaticMesh2`) (`self.StaticMesh3`) (`self.StaticMesh18`) (`self.StaticMesh12`) (`self.StaticMesh20`) (`self.StaticMesh21`) (`self.StaticMesh22`) (`self.StaticMesh23`) (`self.StaticMesh11`) (`self.StaticMesh19`) (`self.StaticMesh14`) (`self.StaticMesh15`) (`self.StaticMesh13`) (`self.StaticMesh16`) (`self.StaticMesh17`))))

(fn `UpdateMat`
  (for _array_element (`self.AllMeshes`)
    (if (not (`KismetArrayLibrary.Array_Contains` (`self.CurrentSelectedMesh`) _array_element))
      (bind _returnvalue (`PrimitiveComponent.CreateDynamicMaterialInstance` _array_element 0 "/Game/Source/Materials/GridShapes/MI_Grid_Flat_Border_Square.MI_Grid_Flat_Border_Square" "None"))
      (`MaterialInstanceDynamic.SetVectorParameterValue` :`self` _returnvalue :`ParameterName` "Color"))))

(fn `UserConstructionScript`)